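; BP_Weapon is a firearm Blueprint that fires automatically while the Shot input is held and manages magazine and reserve ammo.
; Each shot spawns a BP_Bullet and a spark emitter at the BulletPlace socket, then repeats through a Delay loop until release or an empty magazine.
; ChangeMag refills the magazine from the reserve and prints both counts.
; AmmoCharge adds one magazine's worth to the reserve, capped at MagLimit.
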(event `InputAction|Shot`
  (params (Key :type "Key Structure"))
  ;[1 1 1] Shot
  (:`Pressed`
    (set `self.Shooting` true)
    (if (and (> (`self.Bullet Now`) 0) (`self.Shooting`)) :!label _label
      (`|SpawnActorFromClass` "/Game/BP/BP_Bullet.BP_Bullet_C" (`SceneComponent.GetSocketTransform` (`self.Weapon model`) "BulletPlace" "RTS_World") "Undefined" "OverrideRootScale" null null)
      (`GameplayStatics.SpawnEmitterAtLocation` "/Game/InfinityBladeEffects/Effects/FX_Monsters/FX_Monster_Ausar/P_AU_Taunt_sparks.P_AU_Taunt_sparks" (`SceneComponent.GetSocketLocation` (`self.Weapon model`) "BulletPlace") (`SceneComponent.GetSocketRotation` (`self.Weapon model`) "None") (0.1 0.1 0.1))
      (set `self.Bullet Now` (- (`self.Bullet Now`) 1))
      (`KismetSystemLibrary.Delay` (`self.Auto`))
      (goto _label)))
  (:`Released`
    (set `self.Shooting` false)))

(event `Change Mag`
  ;[0.1012 1 0.1344] Change Mag
  (set `self.Mag Charge` (- (`self.Mag Size`) (`self.Bullet Now`)))
  (if (not (>= (`self.Bullet Full`) (`self.Mag Charge`)))
    (set `self.Mag Charge` (`self.Bullet Full`)))
  (set `self.Bullet Now` (+ (`self.Bullet Now`) (`self.Mag Charge`)))
  (set `self.Bullet Full` (- (`self.Bullet Full`) (`self.Mag Charge`)))
  (`KismetSystemLibrary.PrintString` (`KismetStringLibrary.Concat_StrStr` "Bullet Now :" (`KismetStringLibrary.Conv_IntToString` (`self.Bullet Now`)) "Bullet Full" (`KismetStringLibrary.Conv_IntToString` (`self.Bullet Full`)))))

(event `AmmoCharge`
  ;[0.3057 1 0.2258] Ammo Charge
  (bind _output_get (set `self.Bullet Full` (+ (`self.Bullet Full`) (`self.Mag Size`))))
  (set `self.Bullet Full` (`KismetMathLibrary.Clamp` _output_get 0 (`self.Mag Limit`))))

(fn `UserConstructionScript`)